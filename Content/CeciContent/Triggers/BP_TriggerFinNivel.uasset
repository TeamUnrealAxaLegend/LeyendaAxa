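; BP_TriggerFinNivel is an end-of-level trigger that shows the level change screen once the tortillería is done.
; On any actor overlap, it finds the first BP_TriggerTortilleria in the world and sets DoneLevelDay if that trigger's TortilleríaDone flag is true.
; Tick polls DoneLevelDay and, through a DoOnce, creates the UI_ChangeLevel widget and adds it to the viewport a single time.
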(event `self.ReceiveActorBeginOverlap`
  (params (OtherActor :type "Actor Object Reference"))
  (bind _outactors (`GameplayStatics.GetAllActorsOfClass` "/Game/CeciContent/Triggers/BP_TriggerTortilleria.BP_TriggerTortilleria_C"))
  (if (`/Game/CeciContent/Triggers/BP_TriggerTortilleria.TortilleríaDone` (`|GetArrayItem` _outactors))
    (set `self.DoneLevelDay` true)))

(event `self.ReceiveTick`
  (params (DeltaSeconds :type "Float (single-precision)"))
  (if (`self.DoneLevelDay`)
    (`/Engine/EditorBlueprintResources/StandardMacros.DoOnce` false
      (:`Completed`
        (bind _returnvalue (`|CreateWidget` "/Game/CeciContent/GUI/Widgets/UI_ChangeLevel.UI_ChangeLevel_C"))
        (`UserWidget.AddToViewport` _returnvalue 0)))))

(fn `UserConstructionScript`)