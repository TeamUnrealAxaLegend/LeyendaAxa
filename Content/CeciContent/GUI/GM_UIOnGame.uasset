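; Game mode that handles saving and restoring the Axa player character's progress in a single save slot.
; BeginPlay loads an existing BP_SaveGameAxa and applies its transform, water total and four orb values to BP_AxaCharacter.
; The SaveGame event creates the slot if missing, then reloads it and writes the character's current values back.
; Despite the name, its UI_OnGame widget creation is disconnected, as that moved to the character Blueprint.
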(event `self.ReceiveBeginPlay`
  (bind _returnvalue (`GameplayStatics.DoesSaveGameExist` "Save1"))
  (if _returnvalue
    ;[1 1 1] Load Game
    (bind _returnvalue_2 (`GameplayStatics.LoadGameFromSlot` "Save1"))
    (bind _asbp_save_game_axa (cast `/Game/CeciContent/BP_SaveGameAxa` _returnvalue_2))
    (bind _asbp_axa_character (cast `/Game/KikeContent/Animations/BP_AxaCharacter` (`GameplayStatics.GetPlayerCharacter` 0)))
    (`self.K2_SetActorTransform` _asbp_axa_character (`/Game/CeciContent/BP_SaveGameAxa.AxaPosition` _asbp_save_game_axa) false false)
    (set `/Game/KikeContent/Animations/BP_AxaCharacter.TotalWater` (`/Game/CeciContent/BP_SaveGameAxa.TotalWaterDrops` _asbp_save_game_axa) _asbp_axa_character)
    (set `/Game/KikeContent/Animations/BP_AxaCharacter.OrbeNaruto` (`/Game/CeciContent/BP_SaveGameAxa.OrbeNaruto` _asbp_save_game_axa) _asbp_axa_character)
    (set `/Game/KikeContent/Animations/BP_AxaCharacter.OrbeGhost` (`/Game/CeciContent/BP_SaveGameAxa.OrbeGost` _asbp_save_game_axa) _asbp_axa_character)
    (set `/Game/KikeContent/Animations/BP_AxaCharacter.OrbeFloat` (`/Game/CeciContent/BP_SaveGameAxa.OrbeFloat` _asbp_save_game_axa) _asbp_axa_character)
    (set `/Game/KikeContent/Animations/BP_AxaCharacter.OrbeXray` (`/Game/CeciContent/BP_SaveGameAxa.OrbeXray` _asbp_save_game_axa) _asbp_axa_character)))

(event `Save Game`
  (bind _asbp_axa_character (cast `/Game/KikeContent/Animations/BP_AxaCharacter` (`GameplayStatics.GetPlayerCharacter` 0) :!pure true))
  (bind _returnvalue (`GameplayStatics.DoesSaveGameExist` "Save1"))
  (if (not _returnvalue)
    (bind _returnvalue_2 (`GameplayStatics.CreateSaveGameObject` "/Game/CeciContent/BP_SaveGameAxa.BP_SaveGameAxa_C"))
    ;[1 1 1] Save Game
    (`GameplayStatics.SaveGameToSlot` _returnvalue_2 "Save1"))
  (bind _returnvalue_3 (`GameplayStatics.LoadGameFromSlot` "Save1"))
  (bind _asbp_save_game_axa (cast `/Game/CeciContent/BP_SaveGameAxa` _returnvalue_3))
  (set `/Game/CeciContent/BP_SaveGameAxa.TotalWaterDrops` (`/Game/KikeContent/Animations/BP_AxaCharacter.TotalWater` (cast `/Game/KikeContent/Animations/BP_AxaCharacter` (`GameplayStatics.GetPlayerCharacter` 0) :!pure true)) _asbp_save_game_axa)
  (set `/Game/CeciContent/BP_SaveGameAxa.AxaPosition` (`self.GetTransform` _asbp_axa_character) _asbp_save_game_axa)
  (set `/Game/CeciContent/BP_SaveGameAxa.OrbeNaruto` (`/Game/KikeContent/Animations/BP_AxaCharacter.OrbeNaruto` _asbp_axa_character) _asbp_save_game_axa)
  (set `/Game/CeciContent/BP_SaveGameAxa.OrbeGost` (`/Game/KikeContent/Animations/BP_AxaCharacter.OrbeGhost` _asbp_axa_character) _asbp_save_game_axa)
  (set `/Game/CeciContent/BP_SaveGameAxa.OrbeFloat` (`/Game/KikeContent/Animations/BP_AxaCharacter.OrbeFloat` _asbp_axa_character) _asbp_save_game_axa)
  (set `/Game/CeciContent/BP_SaveGameAxa.OrbeXray` (`/Game/KikeContent/Animations/BP_AxaCharacter.OrbeXray` _asbp_axa_character) _asbp_save_game_axa)
  (`GameplayStatics.SaveGameToSlot` _asbp_save_game_axa "Save1"))

(fn `UserConstructionScript`)