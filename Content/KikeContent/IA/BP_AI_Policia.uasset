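; AI controller for the police NPC that detects the player and feeds that to its behavior tree.
; On BeginPlay it runs BT_Policia and caches the possessed BP_Policia pawn.
; Perception updates on the player-controlled BP_AxaCharacter write the CanSeePlayer blackboard key and raise the pawn's walk speed, which is never lowered here, even when sight is lost.
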(event `self.ReceiveBeginPlay`
  (`self.RunBehaviorTree` "/Game/KikeContent/IA/BT_Policia.BT_Policia")
  (bind _asbp_policia (cast `/Game/KikeContent/Animations/NPC/Policia/BP_Policia` (`self.K2_GetPawn`)))
  (set `self.Policia` _asbp_policia))

(event `self.AIPerception.OnTargetPerceptionUpdated`
  (params (Actor :type "Actor Object Reference") (Stimulus :type "AIStimulus Structure"))
  (bind _asbp_axa_character (cast `/Game/KikeContent/Animations/BP_AxaCharacter` Actor))
  (if (`Pawn.IsPlayerControlled` _asbp_axa_character)
    (`BlackboardComponent.SetValueAsBool` (`AIBlueprintHelperLibrary.GetBlackboard` null) "CanSeePlayer" (`.bSuccessfullySensed` (break `AIStimulus` Stimulus)))
    (set `CharacterMovementComponent.MaxWalkSpeed` 1000.0 (`Character.CharacterMovement` (`self.Policia`)))))

(fn `UserConstructionScript`)