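; Llorona conclusion point actor that stays hidden until the player character's Final flag is set, then presents the closing dialogue and cinematic.
; BeginPlay gathers DialoguesAxa rows matching its NPCID; Interact advances the line shown in a Dialogue1 widget and, once only, plays a delayed level sequence.
; Box overlap in the Final state messages overlapping InteractionDialogue actors, and leaving clears the dialogue.
; Tick polls the flag, and EndLevel adds a border widget.
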(event `self.ReceiveBeginPlay`
  (`SceneComponent.SetVisibility` (`self.DefaultSceneRoot`) false true)
  (bind _outrownames (`DataTableFunctionLibrary.GetDataTableRowNames` "/Game/CeciContent/GUI/Dialogues/DialoguesAxa.DialoguesAxa"))
  (for _array_element _outrownames
    (bind _returnvalue (`|GetDataTableRow` "/Game/CeciContent/GUI/Dialogues/DialoguesAxa.DialoguesAxa" _array_element)
      (:`then`
        (if (== (`.NPC_ID_2_D4F65C844D6A856506B545B4723E5BC8` (break `/Game/CeciContent/GUI/Dialogues/DialogueStructure` _returnvalue)) (`self.NPC_ID`))
          (`KismetArrayLibrary.Array_Add` (`self.Dialogue`) _array_element))))))

(event `/Game/CeciContent/GUI/Dialogues/Interaction-Dialogue.Interact`
  (`/Engine/EditorBlueprintResources/StandardMacros.IncrementInt` (`self.Line_ID`)
    (:`  `
      (`self.DialogueCreate`)
      (`/Engine/EditorBlueprintResources/StandardMacros.DoOnce` false
        (:`Completed`
          (`KismetSystemLibrary.Delay` 5.0)
          (bind (_outactor _returnvalue) (`LevelSequencePlayer.CreateLevelSequencePlayer` (`self.Sequence`)))
          (`MovieSceneSequencePlayer.Play` _returnvalue))))))

(event `self.ReceiveTick`
  (params (DeltaSeconds :type "Float (single-precision)"))
  (bind _asbp_axa_character (cast `/Game/KikeContent/Animations/BP_AxaCharacter` (`GameplayStatics.GetPlayerCharacter` 0)))
  (if (`/Game/KikeContent/Animations/BP_AxaCharacter.Final` _asbp_axa_character)
    (`SceneComponent.SetVisibility` (`self.DefaultSceneRoot`) true true)))

(event `self.Box.OnComponentBeginOverlap`
  (params (OverlappedComponent :type "PrimitiveComponent Object Reference") (OtherActor :type "Actor Object Reference") (OtherComp :type "PrimitiveComponent Object Reference") (OtherBodyIndex :type Integer) (bFromSweep :type Boolean) (SweepResult :type "HitResult Structure (by ref)"))
  (bind _asbp_axa_character (cast `/Game/KikeContent/Animations/BP_AxaCharacter` (`GameplayStatics.GetPlayerCharacter` 0)))
  (if (`/Game/KikeContent/Animations/BP_AxaCharacter.Final` _asbp_axa_character)
    (bind _outactors (`GameplayStatics.GetAllActorsWithInterface` "/Game/CeciContent/GUI/Dialogues/Interaction-Dialogue.Interaction-Dialogue_C"))
    (for _array_element _outactors
      (if (`self.IsOverlappingActor` _array_element _asbp_axa_character)
        (message `/Game/CeciContent/GUI/Dialogues/Interaction-Dialogue.Interact` _array_element)))))

(event `self.Box.OnComponentEndOverlap`
  (params (OverlappedComponent :type "PrimitiveComponent Object Reference") (OtherActor :type "Actor Object Reference") (OtherComp :type "PrimitiveComponent Object Reference") (OtherBodyIndex :type Integer))
  (bind _dialoguewidget (`self.DialogueWidget`))
  (`/Engine/EditorBlueprintResources/StandardMacros.IsValid` _dialoguewidget
    (:`Is Valid`
      (`Widget.RemoveFromParent` _dialoguewidget)
      (set `self.DialogueWidget` null)
      (set `self.Line_ID` 0))))

(event `EndLevel`
  (bind _returnvalue (`|CreateWidget` "/Game/KikeContent/UI_GameOverL1/WBP_OutBorder1.WBP_OutBorder1_C"))
  (`UserWidget.AddToViewport` _returnvalue 0))

(fn `DialogueCreate`
  (bind _dialoguewidget (`self.DialogueWidget`))
  (bind _dialoguewidget_2 (`self.DialogueWidget`))
  (`/Engine/EditorBlueprintResources/StandardMacros.IsValid` (`self.DialogueWidget`)
    (:`Is Valid`
      (bind _returnedline (`self.GetDialogue`))
      (`/Engine/EditorBlueprintResources/StandardMacros.IsValid` _dialoguewidget
        (:`Is Valid`
          (set `/Game/CeciContent/GUI/Dialogues/Dialogue1.DialogueText` _returnedline _dialoguewidget))))
    (:`Is Not Valid`
      (bind _returnvalue (`|CreateWidget` "/Game/CeciContent/GUI/Dialogues/Dialogue1.Dialogue1_C" (`GameplayStatics.GetPlayerController` 0)))
      (bind _output_get (set `self.DialogueWidget` _returnvalue))
      (`UserWidget.AddToViewport` _output_get 0)
      (bind _returnedline_2 (`self.GetDialogue`))
      (`/Engine/EditorBlueprintResources/StandardMacros.IsValid` _dialoguewidget_2
        (:`Is Valid`
          (set `/Game/CeciContent/GUI/Dialogues/Dialogue1.DialogueText` _returnedline_2 _dialoguewidget_2))))))

(fn `GetDialogue`
  (returns (ReturnedLine :type Text))
  (locals (ReturnedLines :type "Array of Text"))
  (for _array_element (`self.Dialogue`)
    (bind _returnvalue (`|GetDataTableRow` "/Game/CeciContent/GUI/Dialogues/DialoguesAxa.DialoguesAxa" _array_element)
      (:`then`
        (bind (_npc_id _conversation_id _line_id _dialogue) (break `/Game/CeciContent/GUI/Dialogues/DialogueStructure` _returnvalue))
        (if (and (== _conversation_id (`self.Conversation_ID`)) (== _line_id (`self.Line_ID`)))
          (`KismetArrayLibrary.Array_Add` (`local.ReturnedLines`) _dialogue)))))
  (if (== (`KismetArrayLibrary.Array_Length` (`local.ReturnedLines`)) 1)
    (return (`|GetArrayItem` (`local.ReturnedLines`)))
    (else
      (`Widget.RemoveFromParent` (`self.DialogueWidget`))
      (set `self.DialogueWidget` null)
      (set `self.Line_ID` 0))))

(fn `UserConstructionScript`)