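; BP_Orbe_Naruto is a Naruto orb pickup that starts hidden and is collected when a BP_AxaCharacter overlaps it.
; Collection sets the character's OrbeNaruto flag, shows the matching orb and bar widgets, and plays a cheer montage and sound.
; It then spawns BP_Llorona_Naruto at an offset and a Checkpoint in place, reveals the BP_GotaFinalGhost actors in GotasNext, and destroys itself.
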(event `self.ReceiveBeginPlay`
  (`SceneComponent.SetVisibility` (`self.DefaultSceneRoot`) false true))

(event `self.ReceiveActorBeginOverlap`
  (params (OtherActor :type "Actor Object Reference"))
  (bind _returnvalue (`self.K2_GetActorLocation`))
  (bind _asbp_axa_character (cast `/Game/KikeContent/Animations/BP_AxaCharacter` OtherActor))
  (set `/Game/KikeContent/Animations/BP_AxaCharacter.OrbeNaruto` true _asbp_axa_character)
  (`Widget.SetVisibility` (`/Game/CeciContent/GUI/UI_OnGame.OrbeNaruto` (`/Game/KikeContent/Animations/BP_AxaCharacter.UI:Widget` _asbp_axa_character)) "Visible")
  (`Widget.SetVisibility` (`/Game/CeciContent/GUI/UI_OnGame.CicleBarNaruto` (`/Game/KikeContent/Animations/BP_AxaCharacter.UI:Widget` _asbp_axa_character)) "Visible")
  (`Character.PlayAnimMontage` _asbp_axa_character "/Game/KikeContent/Animations/Abilities/Cheer_AnimMontage.Cheer_AnimMontage" 1.0 "None")
  (`GameplayStatics.PlaySoundAtLocation` "/Game/KikeContent/BP_Points/SkillUp.SkillUp" _returnvalue (struct) 1.0 1.0 0.0 null null null)
  (`|SpawnActorFromClass` "/Game/KikeContent/BP_Points/Naruto/BP_Llorona_Naruto.BP_Llorona_Naruto_C" (`KismetMathLibrary.MakeTransform` (+ _returnvalue (0.0 -200.0 0.0)) (`KismetMathLibrary.Conv_VectorToRotator` (`self.Rotation`))) "Undefined" "OverrideRootScale" null null)
  (`|SpawnActorFromClass` "/Game/CeciContent/Checkpoint.Checkpoint_C" (`self.GetTransform`) "Undefined" "OverrideRootScale" null null)
  (for _array_element (`self.GotasNext`)
    (bind _asbp_gota_final_ghost (cast `/Game/KikeContent/BP_Points/Ghost/BP_GotaFinalGhost` _array_element))
    (`SceneComponent.SetVisibility` (`Actor.RootComponent` _asbp_gota_final_ghost) true true))
  (`self.K2_DestroyActor`))

(fn `UserConstructionScript`)