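; Pickup orb that grants the Float ability to BP_AxaCharacter, starting hidden with collision off.
; A one-time overlap sets the ability flag, shows its UI, plays a cheer montage and sound, and spawns BP_Llorona_Float plus a temporary Checkpoint.
; It then destroys the previous Ghost and Naruto orbs and enables the next BP_GotaFinalXray drops.
; After a short delay, it removes the checkpoint and itself.
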(event `self.ReceiveBeginPlay`
  (`self.SetActorEnableCollision` false)
  (`self.SetActorHiddenInGame` true))

(event `self.ReceiveActorBeginOverlap`
  (params (OtherActor :type "Actor Object Reference"))
  (bind _returnvalue (`self.K2_GetActorLocation`))
  (`/Engine/EditorBlueprintResources/StandardMacros.DoOnce` false
    (:`Completed`
      (bind _asbp_axa_character (cast `/Game/KikeContent/Animations/BP_AxaCharacter` OtherActor))
      (set `/Game/KikeContent/Animations/BP_AxaCharacter.OrbeFloat` true _asbp_axa_character)
      (`Widget.SetVisibility` (`/Game/CeciContent/GUI/UI_OnGame.CicleBarFloat` (`/Game/KikeContent/Animations/BP_AxaCharacter.UI:Widget` _asbp_axa_character)) "Visible")
      (`Widget.SetVisibility` (`/Game/CeciContent/GUI/UI_OnGame.OrbeFloat` (`/Game/KikeContent/Animations/BP_AxaCharacter.UI:Widget` _asbp_axa_character)) "Visible")
      (`Character.PlayAnimMontage` _asbp_axa_character "/Game/KikeContent/Animations/Abilities/Cheer_AnimMontage.Cheer_AnimMontage" 1.0 "None")
      (`GameplayStatics.PlaySoundAtLocation` "/Game/KikeContent/BP_Points/SkillUp.SkillUp" _returnvalue (struct) 1.0 1.0 0.0 null null null)
      (`|SpawnActorFromClass` "/Game/KikeContent/BP_Points/Float/BP_Llorona_Float.BP_Llorona_Float_C" (`KismetMathLibrary.MakeTransform` (+ _returnvalue (0.0 -200.0 0.0)) (`KismetMathLibrary.Conv_VectorToRotator` (`self.Rotation`))) "Undefined" "OverrideRootScale" null null)
      (bind _returnvalue_2 (`|SpawnActorFromClass` "/Game/CeciContent/Checkpoint.Checkpoint_C" (`self.GetTransform`) "Undefined" "OverrideRootScale" null null))
      (bind _asbp_orbe_ghost (cast `/Game/KikeContent/BP_Points/Ghost/BP_Orbe_Ghost` (`self.OrbeAnterior`))
        (:`then`
          (`/Engine/EditorBlueprintResources/StandardMacros.IsValid` _asbp_orbe_ghost
            (:`Is Valid`
              (`self.K2_DestroyActor` _asbp_orbe_ghost))
            (:`Is Not Valid`
              _)))
        (:`CastFailed`
          _))
      (bind _asbp_orbe_naruto (cast `/Game/KikeContent/BP_Points/Naruto/BP_Orbe_Naruto` (`self.OrbeAnteriorx2`))
        (:`then`
          (`/Engine/EditorBlueprintResources/StandardMacros.IsValid` _asbp_orbe_naruto
            (:`Is Valid`
              (`self.K2_DestroyActor` _asbp_orbe_naruto))
            (:`Is Not Valid`
              _)))
        (:`CastFailed`
          _))
      (for _array_element (`self.GotasNext`)
        (bind _asbp_gota_final_xray (cast `/Game/KikeContent/BP_Points/Xray/BP_GotaFinalXray` _array_element))
        (`self.SetActorHiddenInGame` _asbp_gota_final_xray false)
        (`self.SetActorEnableCollision` _asbp_gota_final_xray true))
      (`KismetSystemLibrary.Delay` 0.5)
      (`self.K2_DestroyActor` _returnvalue_2)
      (`self.K2_DestroyActor`))))

(fn `UserConstructionScript`)